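; BP_DummyTarget is a target dummy whose board flips between standing and knocked-down positions.
; EventStandUp and EventDown each play their own timeline that drives the pitch of TargetBoard's relative rotation.
; A CurrentStatus enum gates both events: stand-up runs only from Down and drop only from Up.
; Ready marks the in-transition state, so repeated calls are ignored until the timeline finishes.
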(event `EventStandUp`
  (switch `/Game/MyContents/enum_TargetState` (`self.currentStatus`)
    (:`NewEnumerator2`
      (set `self.currentStatus` "NewEnumerator0")
      (bind (_direction _newtrack_0) (`Timeline|Timeline_up` :!via `PlayFromStart`)
        (:`Update`
          (`SceneComponent.K2_SetRelativeRotation` (`self.TargetBoard`) (`KismetMathLibrary.MakeRotator` 0.0 _newtrack_0) false false))
        (:`Finished`
          (set `self.currentStatus` "NewEnumerator1"))))))

(event `EventDown`
  (switch `/Game/MyContents/enum_TargetState` (`self.currentStatus`)
    (:`NewEnumerator1`
      (set `self.currentStatus` "NewEnumerator0")
      (bind (_direction _newtrack_0) (`Timeline|Timeline_down` :!via `PlayFromStart`)
        (:`Update`
          (`SceneComponent.K2_SetRelativeRotation` (`self.TargetBoard`) (`KismetMathLibrary.MakeRotator` 0.0 _newtrack_0) false false))
        (:`Finished`
          (set `self.currentStatus` "NewEnumerator2"))))))

(fn `UserConstructionScript`)